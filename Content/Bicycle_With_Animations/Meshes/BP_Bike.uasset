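; BP_Bike is a bicycle actor that reacts to Interact when the player is nearby; actual riding is not implemented.
; NearCollision overlaps with BP_ThirdPersonCharacter toggle the actor's input and a Gate, printing Polish proximity messages.
; While the gate is open, Interact prints a "not programmed" notice and flip-flops BikeMesh between upright with physics off and physics simulation on.
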(event `InputAction|Interact`
  (params (Key :type "Key Structure"))
  ;[1 1 1] Krzysztof - Czy gracz jest przy rowerze? Używa NearCollision aby sprawdzić czy gracz jest w pobliżu
  (:`Pressed`
    (`/Engine/EditorBlueprintResources/StandardMacros.Gate` true :!label _label
      (:`Exit`
        (`KismetSystemLibrary.PrintText` "Chcesz wejsc na rowerek? Niestety nie zaprogramowalem tego.")
        (`/Engine/EditorBlueprintResources/StandardMacros.FlipFlop`
          (:`A`
            (`SceneComponent.K2_SetWorldRotation` :`self` (`self.Bike_Mesh`))
            (`PrimitiveComponent.SetSimulatePhysics` (`self.Bike_Mesh`) false))
          (:`B`
            (`PrimitiveComponent.SetSimulatePhysics` (`self.Bike_Mesh`) true)))))))

(event `self.NearCollision.OnComponentBeginOverlap`
  (params (OverlappedComponent :type "PrimitiveComponent Object Reference") (OtherActor :type "Actor Object Reference") (OtherComp :type "PrimitiveComponent Object Reference") (OtherBodyIndex :type Integer) (bFromSweep :type Boolean) (SweepResult :type "HitResult Structure (by ref)"))
  ;[1 1 1] Krzysztof - Czy gracz jest przy rowerze? Używa NearCollision aby sprawdzić czy gracz jest w pobliżu
  (cast `/Game/ThirdPerson/Blueprints/BP_ThirdPersonCharacter` OtherActor)
  (`self.EnableInput` (`GameplayStatics.GetPlayerController` 0))
  (`KismetSystemLibrary.PrintText` "Jestes w poblizu rowerka.")
  (goto _label :!via `Open`))

(event `self.NearCollision.OnComponentEndOverlap`
  (params (OverlappedComponent :type "PrimitiveComponent Object Reference") (OtherActor :type "Actor Object Reference") (OtherComp :type "PrimitiveComponent Object Reference") (OtherBodyIndex :type Integer))
  ;[1 1 1] Krzysztof - Czy gracz jest przy rowerze? Używa NearCollision aby sprawdzić czy gracz jest w pobliżu
  (cast `/Game/ThirdPerson/Blueprints/BP_ThirdPersonCharacter` OtherActor)
  (`self.DisableInput` (`GameplayStatics.GetPlayerController` 0))
  (`KismetSystemLibrary.PrintText` "Jestes daleko od rowerka")
  (goto _label :!via `Close`))

(fn `UserConstructionScript`)